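; BP_EntryHUD is the HUD for the entry screen that displays the main menu.
; CreateMenu adds the MainMenu widget to the viewport, switches the view to the camera tagged MainCamera, shows the mouse cursor and sets UI-only input.
; ShowPasswordBox forwards a session result to the menu widget.
; The event graph does nothing live, holding only unconnected leftovers, including an older copy of the menu setup.
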(event EventBeginPlay)

(event Collision|EventActorBeginOverlap
  (params (OtherActor :type Actor%20Object%20Reference)))

(event EventTick
  (params (DeltaSeconds :type Float%20%28single-precision%29)))

(fn ConstructionScript)

(fn ShowPasswordBox
  (params (SessionResult :type Blueprint%20Session%20Result%20Structure))
  (Default|ShowPasswordBox (Variables|Default|GetHudWidget) SessionResult))

(fn CreateMenu
  (bind _returnvalue (Game|GetPlayerController 0))
  (bind _returnvalue_2 (UserInterface|CreateWidget "/Game/UI/Entry/MainMenu.MainMenu_C" (Game|GetPlayerController 0)))
  (bind _output_get (Variables|Default|SetHudWidget _returnvalue_2))
  (UserInterface|Viewport|AddtoViewport _output_get 0)
  (bind _outactors (Actor|GetAllActorswithTag "MainCamera"))
  (for _array_element _outactors
    (bind _ascamera_actor (Utilities|Casting|CastToCameraActor _array_element))
    (Game|Player|SetViewTargetwithBlend (Game|GetPlayerController 0) _ascamera_actor 0.0 "VTBlend_Linear" 0.0 true)
    (Variables|/Script/Engine.PlayerController|SetbShowMouseCursor _returnvalue true)
    (Input|SetInputModeUIOnly _returnvalue 0 "DoNotLock")))