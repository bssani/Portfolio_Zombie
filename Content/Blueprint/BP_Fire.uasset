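; Campfire actor that the player lights with E to act as a save point, with healing and respawn triggers.
; Inside FireTrigger, E shows the fire and light, starts audio and calls OnSavePoint with the fire's location and random yaw.
; CustomDepth overlap highlights the wood meshes through custom depth until lit.
; RespawnTrigger overlap starts player healing and stores their transform as the game mode's SpawnTransform, whether lit or not.
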(event OnComponentBeginOverlap(FireTrigger)
  (params (OverlappedComponent :type Primitive%20Component%20Object%20Reference) (OtherActor :type Actor%20Object%20Reference) (OtherComp :type Primitive%20Component%20Object%20Reference) (OtherBodyIndex :type Integer) (bFromSweep :type Boolean) (SweepResult :type Hit%20Result%20Structure%20%28by%20ref%29))
  (Input|EnableInput (Game|GetPlayerController 0)))

(event OnComponentEndOverlap(FireTrigger)
  (params (OverlappedComponent :type Primitive%20Component%20Object%20Reference) (OtherActor :type Actor%20Object%20Reference) (OtherComp :type Primitive%20Component%20Object%20Reference) (OtherBodyIndex :type Integer))
  (Input|DisableInput (Game|GetPlayerController 0)))

(event OnComponentBeginOverlap(RespawnTrigger)
  (params (OverlappedComponent :type Primitive%20Component%20Object%20Reference) (OtherActor :type Actor%20Object%20Reference) (OtherComp :type Primitive%20Component%20Object%20Reference) (OtherBodyIndex :type Integer) (bFromSweep :type Boolean) (SweepResult :type Hit%20Result%20Structure%20%28by%20ref%29))
  (bind _asbp_shooting_player (Utilities|Casting|CastToBP_ShootingPlayer OtherActor))
  (Default|CamFireHeal _asbp_shooting_player)
  (bind _asbp_shooting_game_mode (Utilities|Casting|CastToBP_ShootingGameMode (Game|GetGameMode)))
  (Variables|/Game/Shooting/GameMode/BP_ShootingGameMode.BP_ShootingGameMode_C|SetSpawnTransform _asbp_shooting_game_mode (Transformation|GetActorTransform _asbp_shooting_player)))

(event OnComponentBeginOverlap(CustomDepth)
  (params (OverlappedComponent :type Primitive%20Component%20Object%20Reference) (OtherActor :type Actor%20Object%20Reference) (OtherComp :type Primitive%20Component%20Object%20Reference) (OtherBodyIndex :type Integer) (bFromSweep :type Boolean) (SweepResult :type Hit%20Result%20Structure%20%28by%20ref%29))
  (Utilities|Casting|CastToBP_ShootingPlayer OtherActor)
  (if (not (Rendering|IsVisible (Variables|Default|GetFire)))
    (CallFunction|ShowCustomDepth true)))

(event OnComponentEndOverlap(CustomDepth)
  (params (OverlappedComponent :type Primitive%20Component%20Object%20Reference) (OtherActor :type Actor%20Object%20Reference) (OtherComp :type Primitive%20Component%20Object%20Reference) (OtherBodyIndex :type Integer))
  (Utilities|Casting|CastToBP_ShootingPlayer OtherActor)
  (if (not (Rendering|IsVisible (Variables|Default|GetFire)))
    (CallFunction|ShowCustomDepth false)))

(event OnComponentEndOverlap(RespawnTrigger)
  (params (OverlappedComponent :type Primitive%20Component%20Object%20Reference) (OtherActor :type Actor%20Object%20Reference) (OtherComp :type Primitive%20Component%20Object%20Reference) (OtherBodyIndex :type Integer))
  (bind _asbp_shooting_player (Utilities|Casting|CastToBP_ShootingPlayer OtherActor))
  (Default|EndCamFireHeal _asbp_shooting_player))

(event EventBeginPlay
  (Rendering|SetVisibility (Variables|Default|GetFire) false false)
  (Rendering|SetVisibility (Variables|Default|GetSpotLight) false false)
  (Components|Activation|SetActive (Variables|Default|GetAudio) false false))

(event Input|KeyboardEvents|E
  (params (Key :type Key%20Structure :default "None"))
  (:Pressed
    (if (not (Rendering|IsVisible (Variables|Default|GetFire)))
      (Rendering|SetVisibility (Variables|Default|GetFire) true false)
      (Rendering|SetVisibility (Variables|Default|GetSpotLight) true false)
      (Components|Activation|SetActive (Variables|Default|GetAudio) true false)
      (CallFunction|ShowCustomDepth false)
      (Collision|SetCollisionEnabled (Variables|Default|GetCustomDepth) "NoCollision")
      (Default|CallOnSavePoint (Math|Transform|MakeTransform (Transformation|GetWorldLocation (Variables|Default|GetDefaultScene)) (Math|Rotator|MakeRotator 0.0 0.0 (Math|Random|RandomFloatinRange 0.0 3.6e+02)) "1,1,1")))))

(fn ConstructionScript)

(fn ShowCustomDepth
  (params (Depth :type Boolean))
  (Rendering|SetRenderCustomDepth (Variables|Default|GetWood1) Depth)
  (return))