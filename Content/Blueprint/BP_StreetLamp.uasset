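; Street lamp actor whose spot light flickers erratically during play.
; BeginPlay starts an endless Delay loop that waits a short random interval, then sets the SpotLight to a random intensity within a wide range.
; A disconnected alternative that blinks the light's visibility off and on remains in the graph but never runs.
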(event EventBeginPlay
  (Utilities|FlowControl|Delay (Math|Random|RandomFloatinRange 0.0 0.8) :!label _label)
  (Rendering|Components|Light|SetIntensity (Variables|Default|GetSpotLight) (Math|Random|RandomFloatinRange 8e+04 7e+05))
  (goto _label))

(event Collision|EventActorBeginOverlap
  (params (OtherActor :type Actor%20Object%20Reference)))

(event EventTick
  (params (DeltaSeconds :type Float%20%28single-precision%29)))

(fn ConstructionScript)