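; BP_MapMusic is a music zone that crossfades the soundtrack when the player enters or leaves it.
; On MusicZone overlap with the player pawn, it finds BP_MusicManager, fades out CurrentMusicRef and fades in the MusicArray track indexed by SelectTrack.
; On exit, it fades that track out and fades in the array's first track.
; The zone itself never updates CurrentMusicRef.
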(event OnComponentBeginOverlap(MusicZone)
  (params (OverlappedComponent :type Primitive%20Component%20Object%20Reference) (OtherActor :type Actor%20Object%20Reference) (OtherComp :type Primitive%20Component%20Object%20Reference) (OtherBodyIndex :type Integer) (bFromSweep :type Boolean) (SweepResult :type Hit%20Result%20Structure%20%28by%20ref%29))
  (if (== OtherActor (Game|Player|GetPlayerPawn 0))
    (bind _returnvalue (Actor|GetActorOfClass "/Game/Blueprint/BP_MusicManager.BP_MusicManager_C"))
    (Audio|Components|Audio|FadeOut (Variables|/Game/Blueprint/BP_MusicManager.BP_MusicManager_C|GetCurrentMusicRef _returnvalue) 3.0 0.0 "Linear" :!class /Script/Engine.AudioComponent)
    (Audio|Components|Audio|FadeIn (Utilities|Array|Get(acopy) (Variables|/Game/Blueprint/BP_MusicManager.BP_MusicManager_C|GetMusicArray _returnvalue) (Variables|Default|GetSelectTrack)) 3.0 1.0 0.0 "Linear" :!class /Script/Engine.AudioComponent)))

(event OnComponentEndOverlap(MusicZone)
  (params (OverlappedComponent :type Primitive%20Component%20Object%20Reference) (OtherActor :type Actor%20Object%20Reference) (OtherComp :type Primitive%20Component%20Object%20Reference) (OtherBodyIndex :type Integer))
  (if (== OtherActor (Game|Player|GetPlayerPawn 0))
    (bind _returnvalue (Actor|GetActorOfClass "/Game/Blueprint/BP_MusicManager.BP_MusicManager_C"))
    (Audio|Components|Audio|FadeOut (Utilities|Array|Get(acopy) (Variables|/Game/Blueprint/BP_MusicManager.BP_MusicManager_C|GetMusicArray _returnvalue) (Variables|Default|GetSelectTrack)) 3.0 0.0 "Linear" :!class /Script/Engine.AudioComponent)
    (Audio|Components|Audio|FadeIn (Utilities|Array|Get(acopy) (Variables|/Game/Blueprint/BP_MusicManager.BP_MusicManager_C|GetMusicArray _returnvalue)) 3.0 1.0 0.0 "Linear" :!class /Script/Engine.AudioComponent)))

(event EventBeginPlay)

(fn ConstructionScript)