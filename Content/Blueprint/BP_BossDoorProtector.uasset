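; Boss door protector actor that lets the player press F inside its trigger box to switch the Key mesh to a pulsing sign material.
; Box overlap with BP_ShootingPlayer toggles input, prompt text and Key custom depth, plus a looping timer that turns the text toward the camera.
; The first press hides the prompt and plays a sound.
; CustomDepth enables custom depth on StaticMesh with authority; player overlap clears it.
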(event OnComponentBeginOverlap(Box)
  (params (OverlappedComponent :type Primitive%20Component%20Object%20Reference) (OtherActor :type Actor%20Object%20Reference) (OtherComp :type Primitive%20Component%20Object%20Reference) (OtherBodyIndex :type Integer) (bFromSweep :type Boolean) (SweepResult :type Hit%20Result%20Structure%20%28by%20ref%29))
  (Utilities|Casting|CastToBP_ShootingPlayer OtherActor)
  (Rendering|SetVisibility (Variables|Default|GetTextRender) true false)
  (Input|EnableInput (Game|GetPlayerController 0))
  (Rendering|SetRenderCustomDepth (Variables|Default|GetStaticMesh) false)
  (Rendering|SetRenderCustomDepth (Variables|Default|GetKey) (not (Variables|/Script/Engine.SceneComponent|GetbHiddenInGame (Variables|Default|GetTextRender))))
  (Utilities|Time|SetTimerbyFunctionName 0 "TextureRotation" 0.02 true))

(event OnComponentEndOverlap(Box)
  (params (OverlappedComponent :type Primitive%20Component%20Object%20Reference) (OtherActor :type Actor%20Object%20Reference) (OtherComp :type Primitive%20Component%20Object%20Reference) (OtherBodyIndex :type Integer))
  (Utilities|Casting|CastToBP_ShootingPlayer OtherActor)
  (Rendering|SetVisibility (Variables|Default|GetTextRender) false false)
  (Input|DisableInput (Game|GetPlayerController 0))
  (Rendering|SetRenderCustomDepth (Variables|Default|GetKey) false)
  (Utilities|Time|ClearTimerbyFunctionName 0 "TextureRotation"))

(event Custom|ResCustumDepth
  (Rendering|SetRenderCustomDepth (Variables|Default|GetStaticMesh) true))

(event Custom|TextureRotation
  (bind _returnvalue (Game|GetPlayerCameraManager 0))
  (bind _transformcomponent (Variables|/Script/Engine.PlayerCameraManager|GetTransformComponent _returnvalue))
  (bind _returnvalue_2 (Transformation|GetWorldRotation _transformcomponent))
  (Transformation|SetWorldRotation (Variables|Default|GetTextRender) (Math|Rotator|MakeRotator (.roll _returnvalue_2) (* (.pitch _returnvalue_2) -1.0) (+ (.yaw _returnvalue_2) 1.8e+02)) false false))

(event EventBeginPlay
  (Rendering|SetVisibility (Variables|Default|GetTextRender) false false))

(event Collision|EventActorBeginOverlap
  (params (OtherActor :type Actor%20Object%20Reference)))

(event EventTick
  (params (DeltaSeconds :type Float%20%28single-precision%29)))

(event Input|KeyboardEvents|F
  (params (Key :type Key%20Structure :default "None"))
  (bind _textrender (Variables|Default|GetTextRender))
  ;[1 1 1] 머티리얼 바꾸기
  (:Pressed
    (Rendering|SetRenderCustomDepth (Variables|Default|GetKey) false)
    (Rendering|Material|SetMaterial (Variables|Default|GetKey) 0 "/Game/MaterialFunctionCollection/Materials/Materials/Pulse/M_Signs_Pulse.M_Signs_Pulse")
    (if (not (Variables|/Script/Engine.SceneComponent|GetbHiddenInGame _textrender))
      (Development|SetHiddeninGame _textrender true false)
      (Audio|PlaySound2D "/Game/Sounds/Item/itemputon.itemputon" 1.0 1.0 0.0 0 0))))

(fn ConstructionScript)

(fn CustomDepth
  (Networking|SwitchHasAuthority
    (:Authority
      (CallFunction|ResCustumDepth))))