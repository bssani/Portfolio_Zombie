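; BP_WaterFog is a water fog particle effect Blueprint with adjustable material appearance.
; Its construction script creates a dynamic material instance from the material at index 2 of its ParticleSystem component.
; It feeds Blueprint variables for particle colour multiplier, emissive colour, density and opacity multiplier into that instance, so the fog's look is editable through the Blueprint.
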(fn ConstructionScript
  ;[1 1 1] Create a dynamic material instance so we can edit material values via blueprint
  (bind _returnvalue (Rendering|Material|CreateDynamicMaterialInstance (Variables|Default|GetParticleSystem) 2 (Rendering|Material|GetMaterial (Variables|Default|GetParticleSystem) 2) :!class /Script/Engine.PrimitiveComponent))
  (Rendering|Material|SetVectorParameterValue _returnvalue "Particle Colour Multiplier" (Variables|Default|GetParticle%20Colour%20Multiplier) :!class /Script/Engine.MaterialInstanceDynamic)
  (Rendering|Material|SetScalarParameterValue _returnvalue "Emissive Colour" (Variables|Default|GetEmissive%20Colour) :!class /Script/Engine.MaterialInstanceDynamic)
  (Rendering|Material|SetScalarParameterValue _returnvalue "Density" (Variables|Default|GetDensity) :!class /Script/Engine.MaterialInstanceDynamic)
  (Rendering|Material|SetScalarParameterValue _returnvalue "Opacity Multiplier" (Variables|Default|GetOpacity%20Multiplier) :!class /Script/Engine.MaterialInstanceDynamic))