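; BP_Fire is an interactive fire actor, apparently a campfire, that the player lights by pressing E.
; On BeginPlay it hides the Fire component and SpotLight and deactivates its Audio.
; The FireTrigger overlap events enable and disable input for player 0 without checking the overlapping actor.
; Pressing E shows the fire and light and activates the sound, with no logic to extinguish it.
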(event OnComponentBeginOverlap(FireTrigger)
  (params (OverlappedComponent :type Primitive%20Component%20Object%20Reference) (OtherActor :type Actor%20Object%20Reference) (OtherComp :type Primitive%20Component%20Object%20Reference) (OtherBodyIndex :type Integer) (bFromSweep :type Boolean) (SweepResult :type Hit%20Result%20Structure%20%28by%20ref%29))
  (Input|EnableInput (Game|GetPlayerController 0)))

(event OnComponentEndOverlap(FireTrigger)
  (params (OverlappedComponent :type Primitive%20Component%20Object%20Reference) (OtherActor :type Actor%20Object%20Reference) (OtherComp :type Primitive%20Component%20Object%20Reference) (OtherBodyIndex :type Integer))
  (Input|DisableInput (Game|GetPlayerController 0)))

(event EventBeginPlay
  (Rendering|SetVisibility (Variables|Default|GetFire) false false)
  (Rendering|SetVisibility (Variables|Default|GetSpotLight) false false)
  (Components|Activation|SetActive (Variables|Default|GetAudio) false false))

(event Input|KeyboardEvents|E
  (params (Key :type Key%20Structure))
  (:Pressed
    (Rendering|SetVisibility (Variables|Default|GetFire) true false)
    (Rendering|SetVisibility (Variables|Default|GetSpotLight) true false)
    (Components|Activation|SetActive (Variables|Default|GetAudio) true false)))

(fn ConstructionScript)