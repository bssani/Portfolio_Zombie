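; BP_ZombieSpawn spawns a small batch of BP_ZombieCa_Child zombies just above its own location on BeginPlay, each with random yaw.
; The first BP_ShootingPlayer to overlap the referenced Navmesh actor is stored as OtherChar, then OnTargetCatch fires once per ZombieActor entry.
; Code filling ZombieActor from overlapping zombies is disconnected.
; The construction script caches Navmesh scale, but the random position offsets using it are unused.
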(event OnActorBeginOverlap(navmesh)
  (params (OverlappedActor :type Actor%20Object%20Reference) (OtherActor :type Actor%20Object%20Reference))
  (bind _asbp_shooting_player (Utilities|Casting|CastToBP_ShootingPlayer OtherActor))
  (Utilities|IsValid (Variables|Default|GetOtherChar)
    (:Is%20Not%20Valid
      (Development|PrintString (Utilities|GetDisplayName _asbp_shooting_player))
      (Variables|Default|SetOtherChar _asbp_shooting_player)
      (for _array_element (Variables|Default|GetZombieActor)
        (Default|CallOnTargetCatch (Variables|Default|GetOtherChar))))))

(event OnActorEndOverlap(navmesh)
  (params (OverlappedActor :type Actor%20Object%20Reference) (OtherActor :type Actor%20Object%20Reference)))

(event EventBeginPlay
  (bind _returnvalue (Transformation|GetActorLocation))
  (for _index (range 0 2)
    (Game|SpawnActorfromClass "/Game/ZombiePackV1/BP_ZombieCa_Child.BP_ZombieCa_Child_C" (Math|Transform|MakeTransform (Math|Vector|MakeVector (.x _returnvalue) (.y _returnvalue) (+ (.z _returnvalue) 5e+01)) (Math|Rotator|MakeRotator 0.0 0.0 (Math|Random|RandomFloatinRange 0.0 3.6e+02)) "1,1,1") "Undefined" 0 false 0 0)
    (Development|PrintString "Hello")))

(event Collision|EventActorBeginOverlap
  (params (OtherActor :type Actor%20Object%20Reference)))

(event EventTick
  (params (DeltaSeconds :type Float%20%28single-precision%29)))

(fn ConstructionScript
  (bind _navmesh (Variables|Default|Getnavmesh))
  (bind _returnvalue (Transformation|GetActorScale3D _navmesh))
  (Variables|Default|SetNavSizeX (.x _returnvalue))
  (Variables|Default|SetNavSizeY (.y _returnvalue)))