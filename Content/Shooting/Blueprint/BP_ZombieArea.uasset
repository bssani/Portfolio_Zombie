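; BP_ZombieArea tracks the zombies of one area and signals when all of them have died.
; ZombieAddCount raises the expected total, ZombieNumber.
; On BeginPlay it binds to its OnDeathInArea dispatcher, and each death increments ZombieCount.
; When the death count equals the total, it fires the OnZombiesDie dispatcher.
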(event Custom|OnDeathInArea_Event
  (bind _zombiecount (Variables|Default|GetZombieCount))
  (Math|Integer|IncrementInt _zombiecount
    (:%20%20
      (if (== _zombiecount (Variables|Default|GetZombieNumber))
        (Default|CallOnZombiesDie)))))

(event EventBeginPlay
  (EventDispatchers|BindEventtoOnDeathinArea (delegate Custom|OnDeathInArea_Event)))

(event EventTick
  (params (DeltaSeconds :type Float%20%28single-precision%29)))

(fn ConstructionScript)

(fn ZombieAddCount
  (bind _result (Math|Integer|IncrementInt (Variables|Default|GetZombieNumber))
    (:%20%20
      (Development|PrintString (Utilities|String|ToString(Integer) _result) false false))))