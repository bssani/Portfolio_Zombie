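; BP_BossProtectorManager tracks boss key progress and triggers a change on the boss door protectors once every key is counted.
; On BeginPlay it counts all BP_BossKey actors in the level as the required total and caches every BP_BossDoorProtector.
; BossKeyCountAdd increments the collected count and, when it equals the total, calls CustomDepth on each cached protector.
; Debug prints report the counts.
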(event EventBeginPlay
  (Utilities|FlowControl|Sequence
    (:then_0
      (bind _outactors (Actor|GetAllActorsOfClass "/Game/Shooting/Blueprint/BP_BossKey.BP_BossKey_C"))
      (for _array_element _outactors
        (bind _result (Math|Integer|IncrementInt (Variables|Default|GetBossKeyMax))
          (:%20%20
            (Development|PrintString (Utilities|String|Append "bossKey" (Utilities|String|ToString(Integer) _result)))))))
    (:then_1
      (bind _outactors_2 (Actor|GetAllActorsOfClass "/Game/Blueprint/BP_BossDoorProtector.BP_BossDoorProtector_C"))
      (Variables|Default|SetBossProtector _outactors_2))))

(event Collision|EventActorBeginOverlap
  (params (OtherActor :type Actor%20Object%20Reference)))

(event EventTick
  (params (DeltaSeconds :type Float%20%28single-precision%29)))

(fn ConstructionScript)

(fn BossKeyCountAdd
  (bind _bosskeycount (Variables|Default|GetBossKeyCount))
  (bind _result (Math|Integer|IncrementInt _bosskeycount)
    (:%20%20
      (Development|PrintString (Utilities|String|ToString(Integer) _result) false false)
      (if (== _bosskeycount (Variables|Default|GetBossKeyMax))
        (Development|PrintString "커스텀 뎁스")
        (for _array_element (Variables|Default|GetBossProtector)
          (Default|CustomDepth _array_element))))))