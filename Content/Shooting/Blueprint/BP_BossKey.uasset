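; BP_BossKey is a boss key pickup that reveals itself once its linked ZombieArea reports its zombies dead.
; A looping timer then spins and bobs the key, with custom depth enabled.
; Inside its sphere, the player gets input and a camera-facing prompt; pressing F increments BossProtectManager's key count, plays a sound and destroys the key.
; The authority switch and ReqPressF are empty stubs.
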(event OnComponentBeginOverlap(Sphere)
  (params (OverlappedComponent :type Primitive%20Component%20Object%20Reference) (OtherActor :type Actor%20Object%20Reference) (OtherComp :type Primitive%20Component%20Object%20Reference) (OtherBodyIndex :type Integer) (bFromSweep :type Boolean) (SweepResult :type Hit%20Result%20Structure%20%28by%20ref%29))
  (Utilities|Casting|CastToBP_ShootingPlayer OtherActor)
  (Rendering|SetVisibility (Variables|Default|GetTextRender) (Variables|Default|GetIsZombieDispatcher) false)
  (Utilities|Time|SetTimerbyFunctionName 0 "RotationText" 0.02 true)
  (Input|EnableInput (Game|GetPlayerController 0)))

(event OnComponentEndOverlap(Sphere)
  (params (OverlappedComponent :type Primitive%20Component%20Object%20Reference) (OtherActor :type Actor%20Object%20Reference) (OtherComp :type Primitive%20Component%20Object%20Reference) (OtherBodyIndex :type Integer))
  (Utilities|Casting|CastToBP_ShootingPlayer OtherActor)
  (Rendering|SetVisibility (Variables|Default|GetTextRender) false false)
  (Utilities|Time|ClearTimerbyFunctionName 0 "RotationText")
  (Input|DisableInput (Game|GetPlayerController 0)))

(event Custom|OnZombiesDead
  (bind _key (Variables|Default|GetKey))
  (bind _output_get (Variables|Default|SetIsZombieDispatcher true))
  (Rendering|SetVisibility _key _output_get false)
  (Rendering|SetRenderCustomDepth _key _output_get)
  (Utilities|Time|SetTimerbyFunctionName 0 "MoveActor" 0.01 true))

(event Custom|RotationText
  (bind _returnvalue (Game|GetPlayerCameraManager 0))
  (bind _transformcomponent (Variables|/Script/Engine.PlayerCameraManager|GetTransformComponent _returnvalue))
  (bind _returnvalue_2 (Transformation|GetWorldRotation _transformcomponent))
  (Transformation|SetWorldRotation (Variables|Default|GetTextRender) (Math|Rotator|MakeRotator (.roll _returnvalue_2) (* (.pitch _returnvalue_2) -1.0) (+ (.yaw _returnvalue_2) 1.8e+02)) false false))

(event Custom|ReqPressF)

(event Custom|ResPressF
  (bind _bossprotectmanager (Variables|Default|GetBossProtectManager))
  (if (Variables|Default|GetIsZombieDispatcher)
    (Utilities|IsValid _bossprotectmanager
      (:Is%20Valid
        (Default|BossKeyCountAdd _bossprotectmanager)
        (Audio|PlaySound2D "/Game/Sounds/Item/itempickup.itempickup" 1.0 1.0 0.0 0 0)
        (Actor|DestroyActor)))))

(event EventBeginPlay
  (bind _zombiearea (Variables|Default|GetZombieArea))
  (Utilities|IsValid _zombiearea
    (:Is%20Valid
      (EventDispatchers|BindEventtoOnZombiesDie _zombiearea (delegate Custom|OnZombiesDead)))))

(event Input|KeyboardEvents|F
  (params (Key :type Key%20Structure :default "None"))
  (:Pressed
    (Networking|SwitchHasAuthority
      (:Authority
        _)
      (:Remote
        _))
    (CallFunction|ResPressF)))

(fn ConstructionScript)

(fn MoveUpDown
  (params (Tick :type Float%20%28single-precision%29))
  (bind _key (Variables|Default|GetKey))
  (bind _key_2 (Variables|Default|GetKey))
  (bind _speed (Variables|Default|GetSpeed))
  (bind _returnvalue (* Tick _speed))
  (if (Variables|Default|GetIsRight)
    (Transformation|AddRelativeLocation _key (Math|Vector|MakeVector 0.0 0.0 _returnvalue) false false)
    (if (> (.z (Variables|/Script/Engine.SceneComponent|GetRelativeLocation _key_2)) 3e+01)
      (Variables|Default|SetIsRight false))
    (else
      (bind _result (Math|Float|NegateFloat _returnvalue)
        (:%20%20
          (Transformation|AddRelativeLocation _key (Math|Vector|MakeVector 0.0 0.0 _result) false false)
          (if (< (.z (Variables|/Script/Engine.SceneComponent|GetRelativeLocation _key_2)) 0.0)
            (Variables|Default|SetIsRight true)))))))

(fn MoveActor
  (CallFunction|MoveRotation)
  (CallFunction|MoveUpDown 0.01))

(fn MoveRotation
  (Transformation|AddRelativeRotation (Variables|Default|GetKey) (Math|Rotator|MakeRotator 0.0 0.0 (Variables|Default|GetRotation)) false false))