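; BP_ShootingHUD is the HUD for the shooting game mode and owns the W_ShootingHud widget.
; On BeginPlay it creates and displays the widget, then sets player 0 to game-only input with the mouse cursor hidden.
; Its functions are thin pass-throughs to the widget for switching the crosshair by equip and TPP state, switching the boss HP bar and updating boss HP.
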(event EventBeginPlay
  (bind _returnvalue (Game|GetPlayerController 0))
  (bind _returnvalue_2 (UserInterface|CreateWidget "/Game/Shooting/Widget/W_ShootingHud.W_ShootingHud_C"))
  (bind _output_get (Variables|Default|SetShootingWidget _returnvalue_2))
  (UserInterface|Viewport|AddtoViewport _output_get 0)
  (Input|SetInputModeGameOnly _returnvalue)
  (Variables|/Script/Engine.PlayerController|SetbShowMouseCursor _returnvalue false))

(event Collision|EventActorBeginOverlap
  (params (OtherActor :type Actor%20Object%20Reference)))

(event EventTick
  (params (DeltaSeconds :type Float%20%28single-precision%29)))

(fn ConstructionScript)

(fn SwitchTPPCrossHair
  (params (Equip :type Boolean) (IsTPP :type Boolean))
  (Default|SwitchEquipCrosshair (Variables|Default|GetShootingWidget) Equip IsTPP))

(fn SwitchShowHpBar
  (Default|SwitchBossHpBar (Variables|Default|GetShootingWidget)))

(fn SetBossProgressBar
  (params (CurHp :type Float%20%28single-precision%29) (MaxHp :type Float%20%28single-precision%29))
  (Default|SetBossHp (Variables|Default|GetShootingWidget) CurHp MaxHp))