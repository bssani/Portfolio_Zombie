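; BP_ShootingGameMode is the game mode for a shooting game and handles respawning of the player character.
; On BeginPlay it binds to the OnDestroyed event of the first player's BP_ShootingPlayer.
; When that pawn is destroyed, it waits briefly, spawns a replacement at the SpawnTransform variable and has player controller 0 possess it.
; The Respawn event then rebinds to the new pawn, so the cycle repeats.
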(event Custom|On%20Destroyed
  (params (DestroyedActor :type Actor%20Object%20Reference))
  (Utilities|FlowControl|Delay 2.0)
  (bind _returnvalue (Game|SpawnActorfromClass "/Game/Shooting/GameMode/BP_ShootingPlayer.BP_ShootingPlayer_C" (Variables|Default|GetSpawnTransform) "Undefined" 0 0))
  (Pawn|Possess (Game|GetPlayerController 0) _returnvalue)
  (CallFunction|Respawn))

(event Custom|Respawn
  (bind _asbp_shooting_player (Utilities|Casting|CastToBP_ShootingPlayer (Game|GetPlayerCharacter 0)))
  (Game|BindEventtoOnDestroyed _asbp_shooting_player (delegate Custom|On%20Destroyed)))

(event EventBeginPlay
  (bind _asbp_shooting_player (Utilities|Casting|CastToBP_ShootingPlayer (Game|GetPlayerCharacter 0)))
  (Game|BindEventtoOnDestroyed _asbp_shooting_player (delegate Custom|On%20Destroyed)))

(fn ConstructionScript)